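; Placeable skeletal mesh actor, apparently for AR, that shows off looping animations and can be spun on demand.
; On BeginPlay it starts the first animation while a timeline slides it along X and scales it up from zero, then adds the WBP_ARControl widget.
; Next/Previous events cycle the five animations with wrap-around, while rotate events set a flag and signed speed that Tick applies as Scene yaw.
; A second fall-and-scale timeline is never run.
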(event Custom|NextAnimation
  (bind _array (Utilities|Array|MakeArray 0 0 0 0 0))
  (bind _skeletalmesh (Variables|Default|GetSkeletalMesh))
  (if (< (Variables|Default|GetCurrentAnimation) (- (Utilities|Array|Length _array) 1))
    (Math|Integer|IncrementInt (Variables|Default|GetCurrentAnimation)
      (:%20%20
        _))
    (else
      (Variables|Default|SetCurrentAnimation 0)))
  (Components|Animation|SetAnimation _skeletalmesh (Utilities|Array|Get(acopy) _array (Variables|Default|GetCurrentAnimation)))
  (Components|Animation|PlayAnimation _skeletalmesh (Utilities|Array|Get(acopy) _array (Variables|Default|GetCurrentAnimation)) true))

(event Custom|PreviousAnimation
  (bind _array (Utilities|Array|MakeArray 0 0 0 0 0))
  (bind _skeletalmesh (Variables|Default|GetSkeletalMesh))
  (if (> (Variables|Default|GetCurrentAnimation) 0)
    (Math|Integer|DecrementInt (Variables|Default|GetCurrentAnimation)
      (:%20%20
        _))
    (else
      (Variables|Default|SetCurrentAnimation (- (Utilities|Array|Length _array) 1))))
  (Components|Animation|SetAnimation _skeletalmesh (Utilities|Array|Get(acopy) _array (Variables|Default|GetCurrentAnimation)))
  (Components|Animation|PlayAnimation _skeletalmesh (Utilities|Array|Get(acopy) _array (Variables|Default|GetCurrentAnimation)) true))

(event Custom|RotateRight
  (Variables|Default|SetbRotate true)
  (Variables|Default|SetRotationSpeed 2e+02))

(event Custom|RotateLeft
  (Variables|Default|SetbRotate true)
  (Variables|Default|SetRotationSpeed -2e+02))

(event Custom|StopRotation
  (Variables|Default|SetbRotate false))

(event EventBeginPlay
  (bind _array (Utilities|Array|MakeArray 0 0 0 0 0))
  (bind _skeletalmesh (Variables|Default|GetSkeletalMesh))
  (bind _output (Utilities|Array|Get(acopy) _array))
  (Utilities|FlowControl|Sequence
    (:then_0
      (Components|Animation|SetAnimation _skeletalmesh _output)
      (Components|Animation|PlayAnimation _skeletalmesh _output true)
      (Variables|Default|SetCurrentAnimation 0))
    (:then_1
      (Variables|Default|SetStartLocation (Transformation|GetActorLocation))
      (bind _location (Timeline|Timeline_1 PlayFromStart)
        (:Update
          (Transformation|SetActorLocation (Math|Vector|Lerp(Vector) (Variables|Default|GetStartLocation) (+ (Variables|Default|GetStartLocation) "-70.000000,0.000000,0.000000") _location) false false)
          (Transformation|SetActorScale3D (Math|Vector|Lerp(Vector) "0, 0, 0" "1.000000,1.000000,1.000000" _location)))
        (:Finished
          (bind _returnvalue (UserInterface|CreateWidget "/Game/Blueprints/UI/WBP_ARControl.WBP_ARControl_C" 0 self))
          (UserInterface|Viewport|AddtoViewport _returnvalue 0))))))

(event EventTick
  (params (DeltaSeconds :type Float%20%28single-precision%29))
  (if (Variables|Default|GetbRotate)
    (Transformation|AddLocalRotation (Variables|Default|GetScene) (Math|Rotator|MakeRotator 0.0 0.0 (* DeltaSeconds (Variables|Default|GetRotationSpeed))) false false)))

(fn ConstructionScript)