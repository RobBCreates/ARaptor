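; AR game mode that drives the onboarding screen flow for a bird-themed augmented reality experience.
; On BeginPlay it shows the intro widget and caches the AR manager, then completion events open the welcome and bird-choice widgets in turn, each given a reference back to the game mode.
; Raptor selection tells the AR manager to start AR, and a spawn event places a placeable actor at a supplied transform.
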(event Custom|IntroComplete
  (bind _returnvalue (UserInterface|CreateWidget "/Game/Blueprints/UI/WBP_Welcome.WBP_Welcome_C" 0 self))
  (UserInterface|Viewport|AddtoViewport _returnvalue 0))

(event Custom|RaptorSelected
  (Default|StartAR (Variables|Default|GetManagerARRef)))

(event Custom|WelcomeComplete
  (bind _returnvalue (UserInterface|CreateWidget "/Game/Blueprints/UI/WBP_ChooseBird.WBP_ChooseBird_C" 0 self))
  (UserInterface|Viewport|AddtoViewport _returnvalue 0))

(event Custom|SpawnModel
  (params (SpawnTransform :type Transform))
  (Game|SpawnActorfromClass "/Game/Blueprints/Placeable/BP_Placeable.BP_Placeable_C" SpawnTransform "AlwaysSpawn" 0 0))

(event EventBeginPlay
  ;[1 1 1] Spawn Intro Widget
  (bind _returnvalue (UserInterface|CreateWidget "/Game/Blueprints/UI/WBP_Intro.WBP_Intro_C" 0 self))
  (bind _output_get (Variables|Default|SetIntroWidgetRef _returnvalue))
  (UserInterface|Viewport|AddtoViewport _output_get 0)
  (bind _outactors (Actor|GetAllActorsOfClass "/Game/Blueprints/BP_ARManager.BP_ARManager_C"))
  (Variables|Default|SetManagerARRef (Utilities|Array|Get(acopy) _outactors)))

(fn ConstructionScript)