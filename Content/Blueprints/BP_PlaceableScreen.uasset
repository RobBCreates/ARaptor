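; A placeable screen actor that plays a video, animates open as a window, spawns a model, then removes itself.
; On BeginPlay it starts media playback, then steps through delayed stages: a raptor window open animation, followed by a spawn request to BP_GameMode.
; The model uses the screen's transform with a world X offset.
; A timeline then scales the actor to zero and destroys it.
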(event Custom|OpenWindow
  (Components|Animation|PlayAnimation (Variables|Default|GetSkeletalMesh) "/Game/Assets/Meshes/AN_ARaptorWindow_Open.AN_ARaptorWindow_Open" false)
  (Utilities|FlowControl|Delay 7.0)
  (CallFunction|SpawnModel))

(event Custom|SpawnModel
  (bind _returnvalue (Transformation|GetActorTransform))
  (bind (_location _rotation _scale) (Math|Transform|BreakTransform _returnvalue))
  (bind _asbp_game_mode (Utilities|Casting|CastToBP_GameMode (Game|GetGameMode)))
  (Default|SpawnModel _asbp_game_mode (Math|Transform|MakeTransform (- _location "-50.000000,0.000000,0.000000") _rotation _scale))
  (Utilities|FlowControl|Delay 1.0)
  (CallFunction|RemoveSelf))

(event Custom|RemoveSelf
  (bind _scale (Timeline|Timeline_0 PlayFromStart)
    (:Update
      (Transformation|SetActorScale3D (Math|Vector|Lerp(Vector) "1.000000,1.000000,1.000000" "0, 0, 0" _scale)))
    (:Finished
      (Actor|DestroyActor))))

(event EventBeginPlay
  (bind _media (Variables|Default|Getmedia))
  (Media|MediaPlayer|OpenSource _media "/Game/Movies/videoplayback.videoplayback")
  (Media|MediaPlayer|Play _media :!class /Script/MediaAssets.MediaPlayer)
  (Utilities|FlowControl|Delay 1.0)
  (CallFunction|OpenWindow))

(fn ConstructionScript)